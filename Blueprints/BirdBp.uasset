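; Player bird for a Flappy Bird-style game, with physics-driven flapping, score counting and game-over handling.
; Right mouse zeroes the capsule's velocity and applies an upward impulse while movement is allowed.
; The first hit disables flapping, then after a delay saves any new high score, shows the game-over widget and pauses.
; BeginPlay loads or creates the high-score save and adds the HUD.
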(event Custom|IncreaseScore
  (Math|Integer|IncrementInt (Variables|Default|GetScore)
    (:%20%20
      (Audio|PlaySoundatLocation "/Game/Assets/SFX/point.point" (Transformation|GetActorLocation) "0, 0, 0" 1.0 1.0 0.0 0 0 0 0))))

(event EventBeginPlay
  (bind _returnvalue (Game|GetPlayerController 0))
  (Variables|/Script/Engine.PlayerController|SetbShowMouseCursor _returnvalue false)
  (Input|SetInputModeGameOnly _returnvalue false)
  (bind _returnvalue_2 (SaveGame|DoesSaveGameExist "1"))
  (if _returnvalue_2
    (bind _returnvalue_3 (SaveGame|LoadGamefromSlot "1"))
    (bind _ashighscoresave_bp (Utilities|Casting|CastToHighscoresaveBp _returnvalue_3))
    (Variables|Default|SetHighscoresaveref _ashighscoresave_bp)
    (else
      (bind _returnvalue_4 (SaveGame|CreateSaveGameObject "/Game/Blueprints/HighscoresaveBp.HighscoresaveBp_C"))
      (bind _output_get (Variables|Default|SetHighscoresaveref _returnvalue_4))
      (SaveGame|SaveGametoSlot _output_get "1")))
  (bind _returnvalue_5 (UserInterface|CreateWidget "/Game/Blueprints/PlayerHudWidgetBp.PlayerHudWidgetBp_C" 0 self))
  (bind _output_get_2 (Variables|Default|SetPlayerHud _returnvalue_5))
  (UserInterface|Viewport|AddtoViewport _output_get_2 0))

(event Collision|EventActorBeginOverlap
  (params (OtherActor :type Actor%20Object%20Reference)))

(event EventTick
  (params (DeltaSeconds :type Float%20%28single-precision%29))
  (bind _returnvalue (Physics|GetPhysicsLinearVelocity (Variables|Default|GetCapsule) "None"))
  (if (> (.z _returnvalue) 0.0)
    (Physics|AddImpulse (Variables|Default|GetCapsule) "0, 0, 0" "None" false)))

(event Collision|EventHit
  (params (MyComp :type Primitive%20Component%20Object%20Reference) (Other :type Actor%20Object%20Reference) (OtherComp :type Primitive%20Component%20Object%20Reference) (bSelfMoved :type Boolean) (HitLocation :type Vector :default "0, 0, 0") (HitNormal :type Vector :default "0, 0, 0") (NormalImpulse :type Vector :default "0, 0, 0") (Hit :type Hit%20Result%20Structure%20%28by%20ref%29))
  (bind _highscoresaveref (Variables|Default|GetHighscoresaveref))
  (Utilities|FlowControl|DoOnce false
    (:Completed
      (Audio|PlaySoundatLocation "/Game/Assets/SFX/hit.hit" (Transformation|GetActorLocation) "0, 0, 0" 1.0 1.0 0.0 0 0 0 0)
      (Variables|Default|SetCanmove? false)
      (Sprite|SetFlipbook (Variables|Default|GetBird) "/Game/Assets/Character/Bird_Flying.Bird_Flying")
      (Class|PrimitiveComponent|SetConstraintMode (Variables|Default|GetCapsule) "XZPlane")
      (Utilities|FlowControl|Delay 2.0)
      (if (> (Variables|Default|GetScore) (Variables|/Game/Blueprints/HighscoresaveBp.HighscoresaveBp_C|GetSavescore (Variables|Default|GetHighscoresaveref)))
        (Variables|/Game/Blueprints/HighscoresaveBp.HighscoresaveBp_C|SetSavescore _highscoresaveref (Variables|Default|GetScore))
        (SaveGame|SaveGametoSlot _highscoresaveref "1"))
      (bind _returnvalue (UserInterface|CreateWidget "/Game/Blueprints/GameoverBp.GameoverBp_C"))
      (bind _output_get (Variables|Default|SetGameoverhud _returnvalue))
      (Rendering|Components|TextRender|SetText (Variables|/Game/Blueprints/GameoverBp.GameoverBp_C|GetPlayerscore _output_get) (Utilities|Text|ToText(Integer) (Variables|Default|GetScore)))
      (Rendering|Components|TextRender|SetText (Variables|/Game/Blueprints/GameoverBp.GameoverBp_C|Getplayershighscore _output_get) (Utilities|Text|ToText(Integer) (Variables|/Game/Blueprints/HighscoresaveBp.HighscoresaveBp_C|GetSavescore (Variables|Default|GetHighscoresaveref))))
      (UserInterface|Viewport|AddtoViewport _output_get 0)
      (Game|SetGamePaused true))))

(event Input|MouseEvents|RightMouseButton
  (params (Key :type Key%20Structure :default "None"))
  (bind _capsule (Variables|Default|GetCapsule))
  (:Pressed
    (if (Variables|Default|GetCanmove?)
      (Physics|SetPhysicsLinearVelocity _capsule "0, 0, 0" false "None")
      (Physics|AddImpulse _capsule "0.000000,0.000000,350.000000" "None" false)
      (Audio|PlaySoundatLocation "/Game/Assets/SFX/wing.wing" (Transformation|GetActorLocation) "0, 0, 0" 1.0 1.0 0.0 0 0 0 0))))

(fn ConstructionScript)